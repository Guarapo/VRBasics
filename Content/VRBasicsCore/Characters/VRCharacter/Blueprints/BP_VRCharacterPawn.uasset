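; VR player pawn Blueprint that routes motion controller input to locomotion, teleport, menu and widget interaction.
; Both thumbsticks feed the same MovePawnForward and MovePawnRight calls.
; Teleport press and release start and finish destination selection on the matching hand actor, if valid.
; The menu shows only while its button is held, and Interact emulates left mouse clicks through the right hand's widget interaction component.
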(event `InputAxis|MotionControllerThumbLeft_X`
  (params (AxisValue :type "Float (single-precision)"))
  ;[0.2762 1 0.7519] Locomotion Movement Input
  (`self.MovePawnRight` AxisValue))

(event `InputAction|TeleportLeft`
  (params (Key :type "Key Structure"))
  ;[1 0.2766 0.3135] Teleport Movement Input
  (:`Pressed`
    (bind _lefthandactor (`self.LeftHandActor`)
      (:`then`
        (`VRMotionControllerActor.StartTeleportDestination` _lefthandactor))
      (:`else`)))
  (:`Released`
    (bind _lefthandactor_2 (`self.LeftHandActor`)
      (:`then`
        (`VRMotionControllerActor.FinishTeleportDestination` _lefthandactor_2))
      (:`else`))))

(event `InputAxis|MotionControllerThumbLeft_Y`
  (params (AxisValue :type "Float (single-precision)"))
  ;[0.2762 1 0.7519] Locomotion Movement Input
  (`self.MovePawnForward` AxisValue))

(event `InputAxis|MotionControllerThumbRight_X`
  (params (AxisValue :type "Float (single-precision)"))
  ;[0.2762 1 0.7519] Locomotion Movement Input
  (`self.MovePawnRight` AxisValue))

(event `InputAction|TeleportRight`
  (params (Key :type "Key Structure"))
  ;[1 0.2766 0.3135] Teleport Movement Input
  (:`Pressed`
    (bind _righthandactor (`self.RightHandActor`)
      (:`then`
        (`VRMotionControllerActor.StartTeleportDestination` _righthandactor))
      (:`else`)))
  (:`Released`
    (bind _righthandactor_2 (`self.RightHandActor`)
      (:`then`
        (`VRMotionControllerActor.FinishTeleportDestination` _righthandactor_2))
      (:`else`))))

(event `InputAxis|MotionControllerThumbRight_Y`
  (params (AxisValue :type "Float (single-precision)"))
  ;[0.2762 1 0.7519] Locomotion Movement Input
  (`self.MovePawnForward` AxisValue))

(event `InputAction|ShowWidgetMenu`
  (params (Key :type "Key Structure"))
  ;[0.4371 0.3968 1] Display Widget
  (:`Pressed`
    (`self.DisplayWidget` true))
  (:`Released`
    (`self.DisplayWidget` false)))

(event `InputAction|Interact`
  (params (Key :type "Key Structure"))
  ;[1 0.9218 0.4561] WidgetInteract
  (:`Pressed`
    (`WidgetInteractionComponent.PressPointerKey` (`VRMotionControllerActor.GetWidgetInteractionComponent` (`self.RightHandActor`)) "LeftMouseButton"))
  (:`Released`
    (`WidgetInteractionComponent.ReleasePointerKey` (`VRMotionControllerActor.GetWidgetInteractionComponent` (`self.RightHandActor`)) "LeftMouseButton")))

(fn `UserConstructionScript`)